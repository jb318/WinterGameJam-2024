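; BP_Button is a puzzle button that a BP_LotteryBall presses by overlapping its Box.
; The mesh material switches between clicked and unclicked as the ball enters and leaves.
; The first press, gated by DoOnce, unlocks the linked Door, calls its Objective, and uses Index to set the matching challenge-cleared flag on the ObjectiveInstance game instance.
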(event OnComponentBeginOverlap(Box)
  (params (OverlappedComponent :type Primitive%20Component%20Object%20Reference) (OtherActor :type Actor%20Object%20Reference) (OtherComp :type Primitive%20Component%20Object%20Reference) (OtherBodyIndex :type Integer) (bFromSweep :type Boolean) (SweepResult :type Hit%20Result%20Structure%20%28by%20ref%29))
  (bind _returnvalue (Game|GetGameInstance))
  (bind _door (Variables|Default|Getdoor))
  (bind _index (Variables|Default|GetIndex))
  ;[1 1 1] Unlocks Door when ball hits button
  (Utilities|Casting|CastToBP_LotteryBall OtherActor)
  (Rendering|Material|SetMaterial (Variables|Default|GetStaticMesh) 0 "/Game/Puzzles/ButtonClickedMAT_Inst.ButtonClickedMAT_Inst")
  (Utilities|FlowControl|DoOnce false
    (:Completed
      (Class|DoorPortal|UnlockDoor _door)
      (Default|Objective _door)
      (if (== _index 1)
        (bind _asobjective_instance (Utilities|Casting|CastToObjectiveInstance _returnvalue))
        (Variables|/Game/Puzzles/ObjectiveInstance.ObjectiveInstance_C|SetChallenge_1_Cleared _asobjective_instance true)
        (elif (== _index 2)
          (bind _asobjective_instance_2 (Utilities|Casting|CastToObjectiveInstance _returnvalue))
          (Variables|/Game/Puzzles/ObjectiveInstance.ObjectiveInstance_C|SetChallenge_2_Cleared _asobjective_instance_2 true)
          (elif (== _index 3)
            (bind _asobjective_instance_3 (Utilities|Casting|CastToObjectiveInstance _returnvalue))
            (Variables|/Game/Puzzles/ObjectiveInstance.ObjectiveInstance_C|SetChallenge_3_Cleared _asobjective_instance_3 true)))))))

(event OnComponentEndOverlap(Box)
  (params (OverlappedComponent :type Primitive%20Component%20Object%20Reference) (OtherActor :type Actor%20Object%20Reference) (OtherComp :type Primitive%20Component%20Object%20Reference) (OtherBodyIndex :type Integer))
  ;[1 1 1] Unlocks Door when ball hits button
  (Utilities|Casting|CastToBP_LotteryBall OtherActor)
  (Rendering|Material|SetMaterial (Variables|Default|GetStaticMesh) 0 "/Game/Puzzles/ButtonUnclickedMAT_Inst.ButtonUnclickedMAT_Inst"))

(event EventBeginPlay
  ;[1 1 1] Set Material on start
  (Rendering|Material|SetMaterial (Variables|Default|GetStaticMesh) 0 "/Game/Puzzles/ButtonUnclickedMAT_Inst.ButtonUnclickedMAT_Inst"))

(fn ConstructionScript)