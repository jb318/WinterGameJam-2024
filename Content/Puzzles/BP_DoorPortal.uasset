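; Door portal to a challenge map, identified by an ID and a linked map.
; On BeginPlay it clears CanEnter if the game instance's ObjectiveInstance marks the matching challenge (1 to 3) as cleared.
; Overlapping its box passes the linked map to the first-person character and briefly shows a Tutorial3 popup, removed early on exit.
; An Objective event updates the character's objective, then meets it after a short delay.
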(event OnComponentBeginOverlap(Box)
  (params (OverlappedComponent :type Primitive%20Component%20Object%20Reference) (OtherActor :type Actor%20Object%20Reference) (OtherComp :type Primitive%20Component%20Object%20Reference) (OtherBodyIndex :type Integer) (bFromSweep :type Boolean) (SweepResult :type Hit%20Result%20Structure%20%28by%20ref%29))
  ;[1 1 1] Sets Relocation Map
  (bind _asbp_first_person_character (Utilities|Casting|CastToBP_FirstPersonCharacter OtherActor))
  (Variables|/Script/TimeWarpC.TimeWarpCCharacter|SetnewMap _asbp_first_person_character (Variables|Default|GetLinkedMap))
  (bind _returnvalue (UserInterface|CreateWidget "/Game/Widgets/Tutorial3.Tutorial3_C"))
  (bind _output_get (Variables|Default|SetInteractPopup _returnvalue))
  (UserInterface|Viewport|AddtoViewport _output_get 0)
  (Utilities|FlowControl|Delay 3.0)
  (Utilities|IsValid (Variables|Default|GetInteractPopup)
    (:Is%20Valid
      (Widget|RemovefromParent (Variables|Default|GetInteractPopup)))))

(event OnComponentEndOverlap(Box)
  (params (OverlappedComponent :type Primitive%20Component%20Object%20Reference) (OtherActor :type Actor%20Object%20Reference) (OtherComp :type Primitive%20Component%20Object%20Reference) (OtherBodyIndex :type Integer))
  (bind _interactpopup (Variables|Default|GetInteractPopup))
  ;[1 1 1] Sets Relocation Map
  (Utilities|Casting|CastToBP_FirstPersonCharacter OtherActor)
  (Utilities|IsValid _interactpopup
    (:Is%20Valid
      (Widget|RemovefromParent _interactpopup))))

(event Custom|Objective
  (bind _as_bp_first_person_character (Variables|Default|GetAs%20BP%20First%20Person%20Character))
  ;[1 1 1] Updates the objective
  (Default|CallUpdateObjective _as_bp_first_person_character)
  (Utilities|FlowControl|Delay 0.2)
  (Default|MeetObjective _as_bp_first_person_character))

(event EventBeginPlay
  (bind _id (Variables|Default|GetID))
  ;[1 1 1] Checks if door value is true on objective instance to make sure you don't do the same challenge
  (bind _asbp_first_person_character (Utilities|Casting|CastToBP_FirstPersonCharacter (Game|GetPlayerCharacter 0)))
  (Variables|Default|SetAs%20BP%20First%20Person%20Character _asbp_first_person_character)
  (bind _asobjective_instance (Utilities|Casting|CastToObjectiveInstance (Game|GetGameInstance)))
  (if (and (Variables|/Game/Puzzles/ObjectiveInstance.ObjectiveInstance_C|GetChallenge_1_Cleared _asobjective_instance) (== _id 1))
    (Variables|Default|SetcanEnter false)
    (elif (and (Variables|/Game/Puzzles/ObjectiveInstance.ObjectiveInstance_C|GetChallenge_2_Cleared _asobjective_instance) (== _id 2))
      (Variables|Default|SetcanEnter false)
      (elif (and (Variables|/Game/Puzzles/ObjectiveInstance.ObjectiveInstance_C|GetChallenge_3_Cleared _asobjective_instance) (== _id 3))
        (Variables|Default|SetcanEnter false)))))

(fn ConstructionScript)